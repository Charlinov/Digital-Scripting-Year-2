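; MirrorOne is a light-puzzle mirror that reflects incoming light onto other mirrors or an IslandSpirit.
; TakeLightInfo stores the source actor and its position and shows the light cone.
; Each Tick aims the cone along the reflection vector and line-traces to its end, ignoring the source.
; A mirror hit locks CanRotate, passes light onward and fits the cone to the distance; an IslandSpirit hit calls LightPuzzleComplete.
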(event `self.ReceiveTick`
  (params (DeltaSeconds :type "Float (single-precision)"))
  (bind _returnvalue (`self.K2_GetActorLocation`))
  (`self.K2_AddActorWorldRotation` (struct))
  (if (not (== (`KismetMathLibrary.VSize` (`self.LightPosition`)) 0.0))
    ;[1 1 1] Gets the reflective vector. x -1, as it was the opposite direction.
    (bind _output_get (set `self.VectorToLight` (- (`self.LightPosition`) _returnvalue)))
    ;[1 1 1] Adding the reflective vector to the location of the mirror to get a rotation so the light shines along the reflective vector.
    (`SceneComponent.K2_SetWorldRotation` (`self.Cube`) (`KismetMathLibrary.FindLookAtRotation` _returnvalue (+ _returnvalue (* (`KismetMathLibrary.GetReflectionVector` _output_get (`self.GetActorForwardVector`)) -1))) false false)
    ;[1 1 1] Make a raycast which starts at the mirrors location and ends at the end of the light.
    (bind (_outhit _returnvalue_2) (`KismetSystemLibrary.LineTraceSingle` (`SceneComponent.K2_GetComponentLocation` (`self.Mirror`)) (`SceneComponent.K2_GetComponentLocation` (`self.LightCone`)) "TraceTypeQuery1" false (`|MakeArray` (`self.OldLight`)) "None" true (struct :`R` 0.912919 :`B` 1.0 :`A` 1.0) (struct :`G` 0.0832 :`B` 1.0 :`A` 1.0) 0.0))
    ;[1 1 1] If the raycast hits something and the object it hits is the mirror...
    (if _returnvalue_2
      (bind (_bblockinghit _binitialoverlap _time _distance _location _impactpoint _normal _impactnormal _physmat _hitactor) (`GameplayStatics.BreakHitResult` _outhit))
      (bind _asmirror_one (cast `/Game/Blueprints/MirrorOne` _hitactor)
        (:`then`
          (set `self.CanRotate` false)
          (`self.TakeLightInfo` _asmirror_one self)
          ;[1 1 1] Set the scale of the cone to the distance between mirrors divided by 300. 300 is a best approximation from testing as there is no documented conversion from distance to scale.
          (`SceneComponent.SetWorldScale3D` (`self.LightCone`) (`KismetMathLibrary.MakeVector` 0.3 0.3 (/ (`KismetMathLibrary.Vector_Distance` (`self.K2_GetActorLocation` _hitactor) (`self.K2_GetActorLocation`)) 300.0)))
          (bind _rootcomponent (`Actor.RootComponent` _asmirror_one))
          ;[1 1 1] Setting the location of the light to the mirror the light is pointing to.
          (`SceneComponent.K2_SetWorldLocation` (`self.ForwardCube`) (`SceneComponent.K2_GetComponentLocation` _rootcomponent) false false)
          (bind (_returnvalue_roll _returnvalue_pitch _returnvalue_yaw) (`KismetMathLibrary.BreakRotator` (`KismetMathLibrary.FindLookAtRotation` (`SceneComponent.K2_GetComponentLocation` _rootcomponent) (`SceneComponent.K2_GetComponentLocation` (`self.Mirror`)))))
          ;[1 1 1] Setting the rotation of the light to look at this mirror
          (`SceneComponent.K2_SetWorldRotation` (`self.ForwardCube`) (`KismetMathLibrary.MakeRotator` _returnvalue_roll _returnvalue_pitch _returnvalue_yaw) false false))
        (:`CastFailed`
          (bind _asisland_spirit (cast `/Game/Blueprints/IslandSpirit` _hitactor))
          (`/Game/Blueprints/IslandSpirit.LightPuzzleComplete` _asisland_spirit))))))

(fn `TakeLightInfo`
  (params (LightTransform :type "Actor Object Reference"))
  (set `self.OldLight` LightTransform)
  (set `self.LightPosition` (`self.K2_GetActorLocation` LightTransform))
  (`SceneComponent.SetVisibility` (`self.LightCone`) true false))

(fn `UserConstructionScript`)