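; TotemOBJ is a totem puzzle object that accepts two rock actors and reports when both are placed.
; When a Rock1 or Rock2 actor overlaps its Box, it destroys that actor and shows the matching rock component on the totem.
; Once both components are visible, it calls PuzzleComplete on the player's FirstPersonCharacter.
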(event `self.Box.OnComponentBeginOverlap`
  (params (OverlappedComponent :type "PrimitiveComponent Object Reference") (OtherActor :type "Actor Object Reference") (OtherComp :type "PrimitiveComponent Object Reference") (OtherBodyIndex :type Integer) (bFromSweep :type Boolean) (SweepResult :type "HitResult Structure (by ref)"))
  (bind _asrock_1 (cast `/Game/Blueprints/Rock1` OtherActor)
    (:`then`
      (`self.K2_DestroyActor` _asrock_1)
      (`SceneComponent.SetVisibility` (`self.Rock1`) true false))
    (:`CastFailed`
      (bind _asrock_2 (cast `/Game/Blueprints/Rock2` OtherActor))
      (`self.K2_DestroyActor` _asrock_2)
      (`SceneComponent.SetVisibility` (`self.Rock2`) true false)))
  (if (and (`SceneComponent.IsVisible` (`self.Rock1`)) (`SceneComponent.IsVisible` (`self.Rock2`)))
    (bind _asfirst_person_character (cast `/Game/FirstPersonBP/Blueprints/FirstPersonCharacter` (`GameplayStatics.GetPlayerCharacter` 0)))
    (`/Game/FirstPersonBP/Blueprints/FirstPersonCharacter.PuzzleComplete` _asfirst_person_character)))

(fn `UserConstructionScript`)