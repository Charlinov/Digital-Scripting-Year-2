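; PuzzleManager tracks a mushroom colour puzzle and tells the player character when it is solved.
; CheckMushroomBlue raises a blue mushroom counter when given the blue emission material, lowers it otherwise, and prints the count.
; Tick, moved to the post-update tick group on BeginPlay, polls the counter and calls MushroomPuzzleComplete on the FirstPersonCharacter once it reaches eight, with a flag preventing repeats.
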(event `self.ReceiveBeginPlay`
  (`self.SetTickGroup` "TG_PostUpdateWork"))

(event `self.ReceiveTick`
  (params (DeltaSeconds :type "Float (single-precision)"))
  (if (>= (`self.BlueMushrooms`) 8)
    (if (not (`self.IsMushroomPuzzleComplete`))
      (bind _asfirst_person_character (cast `/Game/FirstPersonBP/Blueprints/FirstPersonCharacter` (`GameplayStatics.GetPlayerCharacter` 0)))
      (`/Game/FirstPersonBP/Blueprints/FirstPersonCharacter.MushroomPuzzleComplete` _asfirst_person_character)
      (set `self.IsMushroomPuzzleComplete` true))))

(fn `CheckMushroomBlue`
  (params (MushroomMaterial :type "MaterialInterface Object Reference"))
  (bind _bluemushrooms (`self.BlueMushrooms`))
  (if (== MushroomMaterial "/Game/Materials/BlueEmission.BlueEmission")
    (bind _output_get (set `self.BlueMushrooms` (+ _bluemushrooms 1)))
    (else
      (bind _output_get_2 (set `self.BlueMushrooms` (- _bluemushrooms 1)))))
  (`KismetSystemLibrary.PrintString` (`KismetStringLibrary.Conv_IntToString` _output_get)))

(fn `UserConstructionScript`)