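; Boat actor Blueprint that switches the boat to a repaired state and position when MoveBoat is called.
; MoveBoat teleports the boat and two referenced oar actors to hardcoded world locations and rotations, then swaps the static mesh material to RepairedBoat.
; The event graph and construction script are empty, so MoveBoat must be triggered from outside this Blueprint.
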(fn `MoveBoat`
  (bind _boatoar (`self.BoatOar`))
  (bind _boatoar2 (`self.BoatOar2`))
  (`self.K2_SetActorLocation` (544.0 2366.0 512.0))
  (`self.K2_SetActorRotation` (`KismetMathLibrary.MakeRotator` -3.0 -5.7 -73.0))
  (`self.K2_SetActorLocation` _boatoar (583.0 2147.0 565.0) false false)
  (`self.K2_SetActorRotation` _boatoar (`KismetMathLibrary.MakeRotator` 10.8 28.5 101.0) false)
  (`self.K2_SetActorLocation` _boatoar2 (481.0 2606.0 554.0) false false)
  (`self.K2_SetActorRotation` _boatoar2 (`KismetMathLibrary.MakeRotator` 0.2 31.0 -76.0) false)
  (`PrimitiveComponent.SetMaterial` (`self.StaticMesh`) 0 (`self.RepairedBoat`)))

(fn `UserConstructionScript`)