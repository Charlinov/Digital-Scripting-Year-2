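; Mushroom is a puzzle piece that toggles its mesh material between blue and red emission through ChangeColour.
; When ChangeOtherMushrooms is true, it also flips two linked mushrooms, passing false so the change does not cascade further.
; Each toggled mushroom reports its current material to a MushroomManager through CheckMushroomBlue.
; The event graph is empty, so ChangeColour runs only when called.
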(fn `ChangeColour`
  (params (ChangeOtherMushrooms :type Boolean))
  ;[1 1 1] If the material instance of the object is 'BlueEmission'...
  (if (== (`PrimitiveComponent.GetMaterial` (`self.Mushroom`) 0) (`self.Blue`))
    ;[1 1 1] Change the colour of the object to 'RedEmission'.
    (`PrimitiveComponent.SetMaterial` (`self.Mushroom`) 0 (`self.Red`))
    (else
      ;[1 1 1] If false, change the colour to 'BlueEmission'.
      (`PrimitiveComponent.SetMaterial` (`self.Mushroom`) 0 (`self.Blue`))))
  (if ChangeOtherMushrooms
    (bind _asmushroom (cast `/Game/Blueprints/Mushroom` (`self.OtherMushroom1`)))
    (`self.ChangeColour` _asmushroom false)
    (bind _asmushroom_2 (cast `/Game/Blueprints/Mushroom` (`self.OtherMushroom2`)))
    (`self.ChangeColour` _asmushroom_2 false)
    (bind _asmushroom_manager (cast `/Game/Blueprints/MushroomManager` (`self.PuzzleManager`)))
    (`/Game/Blueprints/MushroomManager.CheckMushroomBlue` _asmushroom_manager (`PrimitiveComponent.GetMaterial` (`self.Mushroom`) 0))
    (else
      (bind _asmushroom_manager_2 (cast `/Game/Blueprints/MushroomManager` (`self.PuzzleManager`)))
      (`/Game/Blueprints/MushroomManager.CheckMushroomBlue` _asmushroom_manager_2 (`PrimitiveComponent.GetMaterial` (`self.Mushroom`) 0)))))

(fn `UserConstructionScript`)